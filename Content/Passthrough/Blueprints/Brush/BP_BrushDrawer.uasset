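; Brush drawer actor that paints strokes in 3D from a VR motion controller and can erase the newest one.
; Starting a stroke spawns a BP_BrushStroke with the brush mesh and material, attaches it to the root and records it in a stack.
; Tick samples the chosen left or right controller on the VRPTPawn, extending the active stroke's spline only after 2 cm of movement.
; Stopping releases the stroke, while erasing pops and destroys the last one.
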(event Custom|StartDrawing
  ;[0.03434 0.03434 0.03434] Input Events - Create & Pop spline
  (CallFunction|CreateSpline (CallFunction|GetDrawPosition)))

(event Custom|StopDrawing
  ;[0.03434 0.03434 0.03434] Input Events - Create & Pop spline
  (CallFunction|CloseSpline))

(event Custom|EraseLastSpline
  ;[0.03434 0.03434 0.03434] Input Events - Create & Pop spline
  (CallFunction|PopSpline))

(event EventTick
  (params (DeltaSeconds :type Float%20%28single-precision%29))
  ;[0.03434 0.03434 0.03434] Tick - Update spline
  (CallFunction|UpdateSpline (CallFunction|GetDrawPosition)))

(fn ConstructionScript)

(fn CreateSpline
  (params (Location :type Vector))
  (bind _returnvalue (Game|SpawnActorfromClass "/Game/Passthrough/Blueprints/Brush/BP_BrushStroke.BP_BrushStroke_C" (Math|Transform|MakeTransform Location "0, 0, 0" "1.000000,1.000000,1.000000") "Undefined" "OverrideRootScale" 0 (Variables|Default|GetBrushMaterial) (Variables|Default|GetBrushMesh) 0))
  (bind _output_get (Variables|Default|SetCurrentBrush _returnvalue))
  (Transformation|AttachComponentToComponent _output_get (Variables|Default|GetDefaultSceneRoot) "None" "KeepRelative" "KeepRelative" "KeepRelative" true)
  (Default|Init _output_get Location)
  (Variables|Default|SetDrawing true)
  (Variables|Default|SetLastLocation Location)
  (Utilities|Array|Add (Variables|Default|GetSplines) _output_get))

(fn UpdateSpline
  (params (Location :type Vector))
  ;[1 1 1] Checks if the distance traveled since last spline point is more than 2 cm and updates spline point if true
  (if (and (> (Math|Vector|Distance(Vector) (Variables|Default|GetLastLocation) Location) 2.0) (Variables|Default|GetDrawing))
    (Default|UpdateSpline (Variables|Default|GetCurrentBrush) Location)
    (Variables|Default|SetLastLocation Location)))

(fn CloseSpline
  (Variables|Default|SetCurrentBrush 0)
  (Variables|Default|SetDrawing false)
  (Variables|Default|SetLastLocation "0, 0, 0"))

(fn PopSpline
  (bind _splines (Variables|Default|GetSplines))
  (bind _returnvalue (Utilities|Array|Length _splines))
  (bind _returnvalue_2 (- _returnvalue 1))
  ;[1 1 1] Removes newest stroke
  (if (> _returnvalue 0)
    (Actor|DestroyActor (Utilities|Array|Get(acopy) _splines _returnvalue_2))
    (Utilities|Array|RemoveIndex _splines _returnvalue_2)))

(fn GetDrawPosition
  (bind _asvrptpawn (Utilities|Casting|CastToVRPTPawn (Game|Player|GetPlayerPawn 0)))
  (return (Transformation|GetWorldLocation (select (Utilities|Enum|Equal(Enum) (Variables|Default|GetDrawOrigin) "Left") (Variables|/Game/Passthrough/Blueprints/VRPTPawn.VRPTPawn_C|GetMotionControllerLeft _asvrptpawn) (Variables|/Game/Passthrough/Blueprints/VRPTPawn.VRPTPawn_C|GetMotionControllerRight _asvrptpawn)))))