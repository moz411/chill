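; BP_BrushStroke is a single brush stroke that grows along a spline as new locations are fed to it.
; Init places the first spline point, then each UpdateSpline call moves or appends a point and advances CurrentIndex.
; Each appended point spawns a spline mesh using BrushMesh and BrushMaterial, built one segment behind the newest point so end tangents orient correctly.
; The construction script is empty, with an unconnected loop that would rebuild segments.
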(fn ConstructionScript)

(fn Init
  (params (Point%20Location :type Vector))
  (Spline|SetLocationatSplinePoint (Variables|Default|GetSpline) 0 Point%20Location "World" true))

(fn UpdateSpline
  (params (New%20Location :type Vector))
  (bind _spline (Variables|Default|GetSpline))
  (bind _spline_2 (Variables|Default|GetSpline))
  (bind _currentindex (Variables|Default|GetCurrentIndex))
  (bind _returnvalue (- _currentindex 2))
  (bind _returnvalue_2 (- _currentindex 1))
  (bind (_location _tangent) (Spline|GetLocationandTangentatSplinePoint _spline _returnvalue "Local"))
  (bind (_location_2 _tangent_2) (Spline|GetLocationandTangentatSplinePoint _spline _returnvalue_2 "Local"))
  ;[1 1 1] Updates/Adds spline point and create a spline mesh. The spline mesh is created one point behind to ensure the rotation of the endpoint of the spline meshes is correct
  (Utilities|FlowControl|Sequence
    (:then_0
      (if (== (Variables|Default|GetCurrentIndex) 1)
        (Spline|SetLocationatSplinePoint _spline_2 (Variables|Default|GetCurrentIndex) New%20Location "World" true)
        (else
          (Spline|AddSplinePoint _spline_2 New%20Location "World" true)
          (bind _returnvalue_3 (AddComponent|AddSplineMeshComponent true))
          (Transformation|AttachComponentToComponent _returnvalue_3 (Variables|Default|GetDefaultSceneRoot) "None" "KeepRelative" "KeepRelative" "KeepRelative" true)
          (Rendering|Material|SetMaterial _returnvalue_3 0 (Variables|Default|GetBrushMaterial))
          (Components|StaticMesh|SetStaticMesh _returnvalue_3 (Variables|Default|GetBrushMesh))
          (SplineMesh|SetStartandEnd _returnvalue_3 _location _tangent _location_2 _tangent_2 true :!class /Script/Engine.SplineMeshComponent))))
    (:then_1
      (Math|Integer|IncrementInt (Variables|Default|GetCurrentIndex)))))