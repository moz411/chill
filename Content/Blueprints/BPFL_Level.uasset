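; Blueprint function library of level helpers for mixed reality rooms built on MRUK.
; It loads random or named rooms from scene-provider JSON, requests Android scene permission, centers actors and fits navmesh bounds to the current room.
; It also toggles global-mesh visibility and collision, and sets materials on tagged procedural meshes of floors, ceilings and visible walls.
; Most current-room or all-room functions delegate to per-room variants.
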(fn ApplyTexturetoWalls
  (for _array_element (Variables|/Script/MRUtilityKit.MRUKSubsystem|GetRooms (Subsystems|GetMRUKSubsystem))
    (CallFunction|ApplyTexturetoWallsinRoom _array_element)))

(fn CenterinCurrentRoom
  (params (Actor :type Actor%20Object%20Reference) (Z :type Float%20%28double-precision%29))
  (CallFunction|CenterinRoom Actor Z (Class|MRUKSubsystem|GetCurrentRoom (Subsystems|GetMRUKSubsystem))))

(fn AdjustNavMeshBounds
  (params (NavMeshBoundsVolume :type Nav%20Mesh%20Bounds%20Volume%20Object%20Reference))
  (Utilities|IsValid (Class|MRUKSubsystem|GetCurrentRoom (Subsystems|GetMRUKSubsystem))
    (:Is%20Valid
      (LocalVariables|SetRoomBounds (Variables|/Script/MRUtilityKit.MRUKRoom|GetRoomBounds (Class|MRUKSubsystem|GetCurrentRoom (Subsystems|GetMRUKSubsystem))))
      (Transformation|SetActorScale3D NavMeshBoundsVolume (+ (/ (- (.max (LocalVariables|GetRoomBounds)) (.min (LocalVariables|GetRoomBounds))) 2.0) 1.0))
      (Transformation|SetActorLocation NavMeshBoundsVolume (/ (+ (.min (LocalVariables|GetRoomBounds)) (.max (LocalVariables|GetRoomBounds))) 2.0) false false)
      (Class|NavigationSystemV1|OnNavigationBoundsUpdated (Class|NavigationSystemV1|GetNavigationSystem) NavMeshBoundsVolume))))

(fn LoadRandomRoom
  (params (SceneDataProvider :type BP%20Scene%20Data%20Provider%20Object%20Reference))
  (bind (_roomjson _roomname) (Class|MRUKSceneDataProvider|GetRoom SceneDataProvider))
  (Class|MRUKSubsystem|LoadScenefromJsonString (Subsystems|GetMRUKSubsystem) _roomjson)
  (Development|PrintText 0 (Utilities|Text|FormatText "Loaded room {name} from JSON" _roomname) true true "(R=0.000000,G=0.660000,B=1.000000,A=1.000000)" 1e+01))

(fn RequestScenePermission
  (bind _returnvalue (Utilities|String|MakeLiteralString "com.oculus.permission.USE_SCENE"))
  (if (Utilities|String|Contains (Game|GetPlatformName) "Android")
    (bind _returnvalue_2 (Class|AndroidPermissionFunctionLibrary|CheckPermission _returnvalue))
    (if _returnvalue_2
      _
      (else
        (bind _returnvalue_3 (Class|AndroidPermissionFunctionLibrary|AcquirePermissions (Utilities|Array|MakeArray _returnvalue)))))
    (return _returnvalue_3 _returnvalue_2)
    (else
      (return 0 false))))

(fn SetGlobalMeshVisible
  (params (Visible :type Boolean))
  (CallFunction|SetGlobalMeshVisibleinRoom (Class|MRUKSubsystem|GetCurrentRoom (Subsystems|GetMRUKSubsystem)) Visible))

(fn EnableGlobalMeshCollision
  (params (Enable :type Boolean))
  (CallFunction|EnableGlobalMeshCollisioninRoom (Class|MRUKSubsystem|GetCurrentRoom (Subsystems|GetMRUKSubsystem)) Enable))

(fn RoomwithGlobalMeshJson
  (params (RoomName :type String) (SceneDataProvider :type BP%20Scene%20Data%20Provider%20Object%20Reference))
  (Variables|/Script/MRUtilityKit.MRUKSceneDataProvider|SetbUseRandomRoom SceneDataProvider false)
  (Variables|/Script/MRUtilityKit.MRUKSceneDataProvider|SetSpecificRoomName SceneDataProvider RoomName)
  (bind _roomjson (Class|MRUKSceneDataProvider|GetRoom SceneDataProvider))
  (return _roomjson))

(fn LoadRoombyName
  (params (RoomName :type Name) (SceneDataProvider :type BP%20Scene%20Data%20Provider%20Object%20Reference))
  (Variables|/Script/MRUtilityKit.MRUKSceneDataProvider|SetbUseRandomRoom SceneDataProvider false)
  (Variables|/Script/MRUtilityKit.MRUKSceneDataProvider|SetSpecificRoomName SceneDataProvider (Utilities|String|ToString(Name) RoomName))
  (bind _roomjson (Class|MRUKSceneDataProvider|GetRoom SceneDataProvider))
  (Class|MRUKSubsystem|LoadScenefromJsonString (Subsystems|GetMRUKSubsystem) _roomjson))

(fn CenterinRoom
  (params (Actor :type Actor%20Object%20Reference) (Z :type Float%20%28double-precision%29) (Room :type MRUK%20Room%20Object%20Reference))
  (bind _returnvalue (Class|MRUKRoom|ComputeCentroid Room Z))
  (Transformation|SetActorLocation Actor _returnvalue false false))

(fn ApplyTexturetoWallsinRoom
  (params (Room :type MRUK%20Room%20Object%20Reference))
  (CallFunction|SetProceduralMeshMaterial (Variables|/Script/MRUtilityKit.MRUKRoom|GetFloorAnchor Room))
  (CallFunction|SetProceduralMeshMaterial (Variables|/Script/MRUtilityKit.MRUKRoom|GetCeilingAnchor Room))
  (for _array_element (Variables|/Script/MRUtilityKit.MRUKRoom|GetWallAnchors Room)
    (if (not (Class|MRUKAnchor|HasLabel _array_element "INVISIBLE_WALL_FACE"))
      (CallFunction|SetProceduralMeshMaterial _array_element))))

(fn SetGlobalMeshVisibleinRoom
  (params (Room :type MRUK%20Room%20Object%20Reference) (Visible :type Boolean))
  (bind _globalmeshanchor (Variables|/Script/MRUtilityKit.MRUKRoom|GetGlobalMeshAnchor Room))
  (Utilities|IsValid Room
    (:Is%20Valid
      (Utilities|IsValid _globalmeshanchor
        (:Is%20Valid
          (Rendering|SetActorHiddenInGame _globalmeshanchor (not Visible)))))))

(fn EnableGlobalMeshCollisioninRoom
  (params (Room :type MRUK%20Room%20Object%20Reference) (Enable :type Boolean))
  (bind _globalmeshanchor (Variables|/Script/MRUtilityKit.MRUKRoom|GetGlobalMeshAnchor Room))
  (Utilities|IsValid Room
    (:Is%20Valid
      (Utilities|IsValid _globalmeshanchor
        (:Is%20Valid
          (Collision|SetActorEnableCollision _globalmeshanchor Enable))))))

(fn SetProceduralMeshMaterial
  (params (Anchor :type MRUK%20Anchor%20Object%20Reference) (Material :type Material%20Interface%20Object%20Reference))
  (for _array_element (Actor|GetAttachedActors Anchor true true)
    (if (Actor|ActorHasTag _array_element "MRUKProceduralAnchorMesh")
      (Rendering|Material|SetMaterial (Actor|GetComponentbyClass _array_element "/Script/ProceduralMeshComponent.ProceduralMeshComponent") 0 Material))))